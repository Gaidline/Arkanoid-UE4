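; KillZone is a level object that destroys balls entering its zone.
; When an actor overlaps the Zone component, it casts to Ball_Base and ignores anything else.
; It destroys the ball, then sends an OnBallDestroyed message to the first player pawn, leaving any further response to that pawn.
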(event OnComponentBeginOverlap(Zone)
  (params (OverlappedComponent :type Primitive%20Component%20Object%20Reference) (OtherActor :type Actor%20Object%20Reference) (OtherComp :type Primitive%20Component%20Object%20Reference) (OtherBodyIndex :type Integer) (bFromSweep :type Boolean) (SweepResult :type Hit%20Result%20Structure%20%28by%20ref%29))
  (bind _asball_base (Utilities|Casting|CastToBall_Base OtherActor))
  (Utilities|FlowControl|Sequence
    (:then_0
      (Actor|DestroyActor _asball_base))
    (:then_1
      (Class|PlayerInterface|OnBallDestroyed(Message) (Game|Player|GetPlayerPawn 0)))))

(event EventBeginPlay
  (|CallParentFunction))

(event Collision|EventActorBeginOverlap
  (params (OtherActor :type Actor%20Object%20Reference))
  (|CallParentFunction OtherActor))

(event EventTick
  (params (DeltaSeconds :type Float%20%28single-precision%29))
  (|CallParentFunction DeltaSeconds))

(fn ConstructionScript
  (|CallParentFunction))