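; DestructibleBox is a level object that a ball can break, built as a grid of boxes in one InstancedStaticMesh.
; AutoArrange rebuilds the grid across Y and down Z, deriving spacing from mesh bounds when either offset is zero.
; DestroyObject removes the given instance, or the whole actor for a negative index.
; GetBounceData keeps the parent's bounce direction and returns this box's own ball speed change.
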(event Custom|Auto%20Arrange
  (bind _num_instances_per_row (Variables|AutoArrangement|GetNum%20Instances%20Per%20Row))
  ;[1 1 1] Auto arrange instances of Destructible Box
  (Utilities|FlowControl|Sequence
    (:then_0
      (Components|InstancedStaticMesh|ClearInstances (Variables|Default|GetInstancedStaticMesh))
      (if (or (== (Variables|AutoArrangement|GetColumns%20Offset) 0.0) (== (Variables|AutoArrangement|GetRows%20Offset) 0.0))
        (CallFunction|CalculateInstancesDefaultOffset)))
    (:then_1
      (for _index (range 0 (- (Variables|AutoArrangement|GetNum%20Instances) 1))
        (bind _returnvalue (Components|InstancedStaticMesh|AddInstance (Variables|Default|GetInstancedStaticMesh) (Math|Transform|MakeTransform (Math|Vector|MakeVector 0.0 (* (Math|Integer|%(Integer) _index _num_instances_per_row) (Variables|AutoArrangement|GetColumns%20Offset)) (* (* (/ _index _num_instances_per_row) (Variables|AutoArrangement|GetRows%20Offset)) -1.0)) "0.000000, 0, 0" "1,1,1")))
        (Development|PrintString (Utilities|String|ToString(Integer) _returnvalue))))))

(event Custom|Calculate%20Instances%20Default%20Offset
  (bind _instancedstaticmesh (Variables|Default|GetInstancedStaticMesh))
  (bind _staticmesh (Variables|/Script/Engine.StaticMeshComponent|GetStaticMesh _instancedstaticmesh))
  (bind _returnvalue (StaticMesh|GetBoundingBox _staticmesh))
  (bind _returnvalue_2 (* (.max _returnvalue) 2.1))
  (bind (_x _y _z) (Math|Vector|BreakVector _returnvalue_2))
  ;[1 1 1] Calculate instances default offset
  (Variables|AutoArrangement|SetColumns%20Offset _y)
  (Variables|AutoArrangement|SetRows%20Offset _z))

(event EventBeginPlay
  ;[0.2594 0.7969 0.1249] Begin
  (|CallParentFunction))

(event EventDestroyObject
  (params (Instance%20Idx :type Integer))
  ;[1 1 1] Destroy Actor after Ball hit
  (if (>= Instance%20Idx 0)
    (bind _returnvalue (Class|InstancedStaticMeshComponent|RemoveInstance (Variables|Default|GetInstancedStaticMesh) Instance%20Idx))
    (Development|PrintString (Utilities|String|Append (Utilities|String|ToString(Integer) Instance%20Idx) ": " (Utilities|String|ToString(Boolean) _returnvalue)))
    (else
      (Actor|DestroyActor))))

(fn ConstructionScript
  (|CallParentFunction))

(fn GetBounceData
  (params (Hit%20Location :type Vector :default "0, 0, 0"))
  (bind _bounce_out_direction (|CallParentFunction Hit%20Location))
  (return _bounce_out_direction (Variables|Default|GetBall%20Speed%20Delta%20On%20Hit)))