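; Player paddle pawn for a Breakout-style game, which also runs the match state, health, points and HUD.
; It spawns an attached ball, launches it on Paddle Kick during play, and respawns it on loss until health runs out.
; Play starts after a timed delay and ends when health or tracked destructible boxes run out.
; GetBounceData maps the hit's offset from paddle center to a clamped bounce angle, steering the ball.
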(event Custom|Init%20Player
  (bind _paddle_mesh (Variables|Default|GetPaddle%20Mesh))
  (Utilities|FlowControl|Sequence
    (:then_0
      ;[1 1 1] Spawn Ball
      (bind _returnvalue (Game|SpawnActorfromClass "/Game/Blueprints/Ball/Ball_Base.Ball_Base_C" (Math|Transform|MakeTransform (Transformation|GetWorldLocation (Variables|Default|GetBall%20Start%20Location)) "0, 0, 0" "0.100000,0.100000,0.100000") "Undefined" 0 0))
      (bind _output_get (Variables|Default|SetBall _returnvalue))
      (Transformation|AttachActorToActor _output_get self "None" "KeepWorld" "KeepWorld" "KeepWorld" true)
      (Variables|Default|SetIs%20Ball%20On%20Standby true))
    (:then_1
      ;[1 1 1] Calculate Paddle mesh extends
      (Variables|Default|SetPaddle%20Mesh%20Extends%20Scaled (* (.max (StaticMesh|GetBoundingBox (Variables|/Script/Engine.StaticMeshComponent|GetStaticMesh _paddle_mesh))) (Variables|/Script/Engine.SceneComponent|GetRelativeScale3D _paddle_mesh))))))

(event Custom|Start%20Game%20Play
  ;[1 1 1] Start game play after few seconds
  (bind _output_get (Variables|Default|SetCurrent%20Game%20State "NewEnumerator1"))
  (Default|UpdateGameHUD (Variables|Default|GetPlayer%20HUD) _output_get)
  (Input|EnableInput (Variables|Default|GetPlayer%20Controller)))

(event Custom|On%20Game%20Over
  (params (Success :type Boolean))
  ;[1 1 1] On game over
  (bind _output_get (Variables|Default|SetCurrent%20Game%20State "NewEnumerator2"))
  (Default|UpdateGameHUD (Variables|Default|GetPlayer%20HUD) _output_get))

(event EventBeginPlay
  ;[0.1442 0.7812 0.03162] Begin
  (Utilities|FlowControl|Sequence
    (:then_0
      ;[1 1 1] Init
      (bind _asplayer_controller (Utilities|Casting|CastToPlayerController (Pawn|GetController)))
      (bind _output_get (Variables|Default|SetPlayer%20Controller _asplayer_controller))
      (Input|DisableInput _output_get)
      (CallFunction|InitPlayer))
    (:then_1
      ;[1 1 1] Gather all Destructible Boxes from level
      (bind _outactors (Actor|GetAllActorsOfClass "/Game/Blueprints/LevelObjects/DestructibleBox.DestructibleBox_C"))
      (Variables|Default|SetDestructible%20Boxes _outactors))
    (:then_2
      ;[1 1 1] Create Player HUD
      (bind _returnvalue (UserInterface|CreateWidget "/Game/Blueprints/Widgets/Player_HUD.Player_HUD_C"))
      (bind _output_get_2 (Variables|Default|SetPlayer%20HUD _returnvalue))
      (UserInterface|Viewport|AddtoViewport _output_get_2 0)
      ;[1 1 1] Start game play after few seconds
      (Utilities|Time|SetTimerbyEvent (delegate Custom|Start%20Game%20Play) 3.0))))

(event EventUpdateCurrentPoints
  (params (Points%20Delta :type Integer))
  ;[1 1 1] Update Player points
  (Variables|Default|SetCurrent%20Points (+ Points%20Delta (Variables|Default|GetCurrent%20Points))))

(event EventOnDestructibleBoxInstancesCleared
  (params (Cleared%20Destructible%20Box :type Destructible%20Box%20Object%20Reference))
  (bind _destructible_boxes (Variables|Default|GetDestructible%20Boxes))
  ;[1 1 1] On all Destructible Boxes destroyed
  (Utilities|Array|RemoveItem _destructible_boxes Cleared%20Destructible%20Box)
  (if (<= (Utilities|Array|Length _destructible_boxes) 0)
    (Components|Movement|StopMovementImmediately (Variables|/Game/Blueprints/Ball/Ball_Base.Ball_Base_C|GetProjectileMovement (Variables|Default|GetBall)))
    (CallFunction|OnGameOver true)))

(event EventOnBallDestroyed
  ;[1 1 1] On Ball destroyed
  (bind _result (Math|Float|DecrementFloat (Variables|Default|GetCurrent%20Health%20Points))
    (:%20%20
      (if (<= _result 0.0)
        (CallFunction|OnGameOver false)
        (else
          (CallFunction|InitPlayer))))))

(event Input|ActionEvents|InputActionPaddleKick
  (params (Key :type Key%20Structure))
  (:Pressed
    (switch Utilities|FlowControl|Switch|SwitchonGameStates (Variables|Default|GetCurrent%20Game%20State)
      (:NewEnumerator1
        ;[1 1 1] Fire Ball
        (if (Variables|Default|GetIs%20Ball%20On%20Standby)
          (bind _ball (Variables|Default|GetBall)
            (:then
              (Transformation|DetachFromActor _ball "KeepWorld" "KeepWorld" "KeepWorld")
              (Default|ToggleMovement _ball true "0,0.600000,0.600000"))
            (:else))))
      (:NewEnumerator2
        ;[1 1 1] Reload Level 1
        (Game|OpenLevel(byName) "Level_1")))))

(event Input|ActionEvents|InputActionExit
  (params (Key :type Key%20Structure))
  ;[1 1 1] Exit game
  (:Pressed
    (Game|QuitGame 0 "Quit")))

(event Input|AxisEvents|InputAxisMoveRight
  (params (AxisValue :type Float%20%28single-precision%29))
  ;[1 1 1] Input Movement
  (switch Utilities|FlowControl|Switch|SwitchonGameStates (Variables|Default|GetCurrent%20Game%20State)
    (:NewEnumerator1
      (Pawn|Input|AddMovementInput "0,1.000000, 0" AxisValue false))))

(fn ConstructionScript)

(fn GetBounceData
  (params (Hit%20Location :type Vector :default "0, 0, 0"))
  (bind _returnvalue (Transformation|GetActorLocation))
  (bind _returnvalue_2 (- Hit%20Location _returnvalue))
  (bind _y (Math|Vector|BreakVector _returnvalue_2))
  (return (Math|Vector|RotateVectorAroundAxis (Math|Vector|MakeVector 0.0 0.0 1.0) (Math|Float|MapRangeClamped (Math|Float|Absolute(Float) _y) 0.0 (.y (Variables|Default|GetPaddle%20Mesh%20Extends%20Scaled)) 0.0 (* (Math|Float|MakeLiteralFloat 75.0) (Math|Float|Sign(Float) _y))) "-1.000000, 0, 0") (Variables|Default|GetBall%20Speed%20Delta%20On%20Hit)))

(fn GetCurrentHP
  (return (Math|Float|Truncate (Variables|Default|GetCurrent%20Health%20Points))))

(fn GetCurrentPoints
  (return (Variables|Default|GetCurrent%20Points)))