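; Base ball actor that moves with a ProjectileMovement component and bounces off the actors its sphere overlaps, adjusting speed on each hit.
; On overlap it reflects velocity about the impact normal and applies the other actor's speed delta, clamped between initial and max speed.
; Hit actors can override the exit direction through bounce data and then receive a destroy message.
; Events reset speed and toggle movement with a launch direction.
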(event OnComponentBeginOverlap(Sphere)
  (params (OverlappedComponent :type Primitive%20Component%20Object%20Reference) (OtherActor :type Actor%20Object%20Reference) (OtherComp :type Primitive%20Component%20Object%20Reference) (OtherBodyIndex :type Integer) (bFromSweep :type Boolean) (SweepResult :type Hit%20Result%20Structure%20%28by%20ref%29))
  (bind (_bblockinghit _binitialoverlap _time _location _impactpoint _normal _impactnormal) (Collision|BreakHitResult SweepResult))
  (bind _projectilemovement (Variables|Default|GetProjectileMovement))
  (bind (_bounce_out_direction _ball_speed_delta) (Class|InteractableInterface|GetBounceData(Message) OtherActor _location))
  (Utilities|FlowControl|Sequence
    (:then_0
      (Variables|/Script/Engine.MovementComponent|SetVelocity _projectilemovement (- (/ (Variables|/Script/Engine.MovementComponent|GetVelocity _projectilemovement) (Variables|Default|GetCurrent%20Speed)) (* (* _impactnormal 2.0) (Math|Vector|DotProduct (/ (Variables|/Script/Engine.MovementComponent|GetVelocity _projectilemovement) (Variables|Default|GetCurrent%20Speed)) _impactnormal)))))
    (:then_1
      (bind _output_get (Variables|Default|SetCurrent%20Speed (Math|Float|Clamp(Float) (+ (Variables|Default|GetCurrent%20Speed) _ball_speed_delta) (Variables|/Script/Engine.ProjectileMovementComponent|GetInitialSpeed _projectilemovement) (Variables|/Script/Engine.ProjectileMovementComponent|GetMaxSpeed _projectilemovement))))
      (if (Math|Vector|NotEqual(Vector) _bounce_out_direction "0, 0, 0" 0.0001) ; Should use externally calculated velocity?
        (Variables|/Script/Engine.MovementComponent|SetVelocity _projectilemovement (* _bounce_out_direction _output_get))
        (else
          (Variables|/Script/Engine.MovementComponent|SetVelocity _projectilemovement (* (Variables|/Script/Engine.MovementComponent|GetVelocity _projectilemovement) _output_get)))))
    (:then_2
      (Class|InteractableInterface|DestroyObject(Message) OtherActor))))

(event Custom|Toggle%20Movement
  (params (Enable :type Boolean) (Start%20Direction%20Normalized :type Vector))
  (bind _projectilemovement (Variables|Default|GetProjectileMovement))
  ;[1 1 1] Toggle Movement
  (if Enable
    (Variables|/Script/Engine.MovementComponent|SetVelocity _projectilemovement (* Start%20Direction%20Normalized (Variables|Default|GetCurrent%20Speed)))
    (Components|Activation|Activate _projectilemovement false)
    (else
      (Variables|/Script/Engine.MovementComponent|SetVelocity _projectilemovement "0, 0, 0")
      (Components|Activation|Deactivate _projectilemovement))))

(event Custom|Reset%20Speed
  ;[1 1 1] Reset current speed
  (Variables|Default|SetCurrent%20Speed (Variables|/Script/Engine.ProjectileMovementComponent|GetInitialSpeed (Variables|Default|GetProjectileMovement))))

(event EventBeginPlay
  (CallFunction|ResetSpeed))

(fn ConstructionScript)